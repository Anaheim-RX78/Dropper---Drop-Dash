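; BP_WinPlatform is the goal platform that ends the game in victory when the MainCharacter hits it.
; Its static mesh hit event plays a victory sound, switches to UI-only input, shows the end game widget and mouse cursor.
; It then sets IsGameOver on the DropperGameInstance, printing an error if that cast fails.
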(event OnComponentHit(StaticMesh)
  (params (HitComponent :type Primitive%20Component%20Object%20Reference) (OtherActor :type Actor%20Object%20Reference) (OtherComp :type Primitive%20Component%20Object%20Reference) (NormalImpulse :type Vector :default "0, 0, 0") (Hit :type Hit%20Result%20Structure%20%28by%20ref%29))
  (bind _returnvalue (Game|GetPlayerController 0))
  (Utilities|Casting|CastToMainCharacter OtherActor)
  (Audio|PlaySound2D "/Game/Level/MainMap/Sounds/SND_Victory_Cue.SND_Victory_Cue" 1.0 1.0 0.0 0 0)
  (Input|SetInputModeUIOnly _returnvalue 0 "LockInFullscreen" false)
  (bind _returnvalue_2 (UserInterface|CreateWidget "/Game/Level/MainMap/UI/BP_WidgetEndGame.BP_WidgetEndGame_C" _returnvalue))
  (UserInterface|Viewport|AddtoViewport _returnvalue_2 0)
  (Variables|/Script/Engine.PlayerController|SetbShowMouseCursor _returnvalue true)
  (bind _asdropper_game_instance (Utilities|Casting|CastToDropperGameInstance (Game|GetGameInstance))
    (:then
      (Variables|/Script/Dropper.DropperGameInstance|SetIsGameOver _asdropper_game_instance true))
    (:CastFailed
      (Development|PrintString "Game instance is not an instance of DropperGameInstance" true true "(R=1.000000,G=0.000000,B=0.000000,A=1.000000)"))))

(event EventBeginPlay)

(event Collision|EventActorBeginOverlap
  (params (OtherActor :type Actor%20Object%20Reference)))

(event EventTick
  (params (DeltaSeconds :type Float%20%28single-precision%29)))

(fn ConstructionScript)